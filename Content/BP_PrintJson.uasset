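; BP_PrintJson is a small test Blueprint that exercises JSON-to-struct conversion and back, printing the results at BeginPlay.
; It parses a hardcoded user record, including a nested item array and an empty list, into the MyUser struct with Json2Struct.
; On success it serializes the struct back through Struct2Json and prints the compact string.
; A second sequence step prints the first Bag item's name if that index is valid.
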(event EventBeginPlay
  (bind _myuser (Variables|Default|GetMyUser))
  (bind _bag (Utilities|Struct|BreakSTRUCT_User _myuser))
  (Utilities|FlowControl|Sequence
    (:then_0
      (bind _returnvalue (Class|Struct2JsonLibaray|Json2Struct "{\"Name\":\"WarriorDan\",\"Age\":7,\"Level\":99,\"XP\":9999999,\"HP\":100,\"Bag\":[{\"ItemType\":7,\"ItemName\":\"BlackSword\"},{\"ItemType\":3,\"ItemName\":\"Water\"}],\"EmptyList\":[]} " (Variables|Default|GetMyUser)))
      (if _returnvalue
        (bind (_jsonstr _returnvalue_2) (Class|Struct2JsonLibaray|Struct2Json (Variables|Default|GetMyUser) false))
        (if _returnvalue_2
          (Development|PrintString _jsonstr))))
    (:then_1
      (if (Utilities|Array|IsValidIndex _bag)
        (Development|PrintString (Utilities|String|ToString(Text) (.ItemName (Utilities|Struct|BreakSTRUCT_BagItem (Utilities|Array|Get(acopy) _bag)))))))))

(fn ConstructionScript)